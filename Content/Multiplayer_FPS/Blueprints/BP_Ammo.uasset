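; BP_Ammo is an ammo pickup actor in a multiplayer FPS that refills ammo for actors that overlap it.
; On sphere overlap, it checks the other actor for the BI_Damage interface and sends it AddAmmoMessage with the recover amount.
; After a brief delay it hides itself and disables collision, then reappears with query-only collision after a few seconds, acting as a timed respawn without destroying the actor.
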(event OnComponentBeginOverlap(Sphere1)
  (params (OverlappedComponent :type Primitive%20Component%20Object%20Reference) (OtherActor :type Actor%20Object%20Reference) (OtherComp :type Primitive%20Component%20Object%20Reference) (OtherBodyIndex :type Integer) (bFromSweep :type Boolean) (SweepResult :type Hit%20Result%20Structure%20%28by%20ref%29))
  (bind _sphere1 (Variables|Default|GetSphere1))
  (if (Utilities|DoesObjectImplementInterface OtherActor "/Game/Multiplayer_FPS/Blueprints/BI_Damage.BI_Damage_C")
    (Class|BIDamage|AddAmmo(Message) OtherActor (Variables|Default|GetAmmo%20recover%20Amount))
    (Utilities|FlowControl|Delay 0.2)
    (Rendering|SetVisibility (Variables|Default|GetDefaultSceneRoot self) false true)
    (Collision|SetCollisionEnabled _sphere1 "NoCollision")
    (Utilities|FlowControl|Delay 5.0)
    (Collision|SetCollisionEnabled _sphere1 "QueryOnly")
    (Rendering|SetVisibility (Variables|Default|GetDefaultSceneRoot) true true)))

(event EventBeginPlay)

(event Collision|EventActorBeginOverlap
  (params (OtherActor :type Actor%20Object%20Reference)))

(event EventTick
  (params (DeltaSeconds :type Float%20%28single-precision%29)))

(fn ConstructionScript)