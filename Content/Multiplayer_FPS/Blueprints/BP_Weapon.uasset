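; Multiplayer FPS weapon that fires a hitscan shot from the shooting character's camera.
; Shoot multicasts directly on authority, while remote callers route through a server RPC to the same multicast.
; The multicast runs a debug-drawn Visibility trace out to the WeaponData range, ignoring the shooter.
; Blocking hits spawn a Niagara burst and send a BI_Damage message to implementing actors, all inside the multicast rather than server-only.
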(event Custom|Shoot
  (params (Object :type Object%20Object%20Reference))
  ;[1 1 1] Shoot
  (Networking|SwitchHasAuthority
    (:Authority
      (CallFunction|RPCShootMC Object))
    (:Remote
      (CallFunction|RPCShootServer Object))))

(event Custom|RPC_Shoot_Server
  (params (Object :type Object%20Object%20Reference))
  (CallFunction|RPCShootMC Object))

(event Custom|RPC_Shoot_MC
  (params (Object :type Object%20Object%20Reference))
  (Development|PrintString (Utilities|GetDisplayName (Components|GetOwner)))
  (bind _asbp_character (Utilities|Casting|CastToBP_Character Object))
  (bind _outhit (Collision|LineTraceByChannel (Transformation|GetWorldLocation (Variables|/Game/Multiplayer_FPS/Blueprints/BP_Character.BP_Character_C|GetFPS%20camera _asbp_character)) (+ (Transformation|GetWorldLocation (Variables|/Game/Multiplayer_FPS/Blueprints/BP_Character.BP_Character_C|GetFPS%20camera _asbp_character)) (* (Math|Vector|GetForwardVector (Transformation|GetWorldRotation (Variables|/Game/Multiplayer_FPS/Blueprints/BP_Character.BP_Character_C|GetFPS%20camera _asbp_character))) (.OutRange (Class|Weapon|SplitWeaponData (Variables|Default|GetWeaponData))))) "TraceTypeQuery1" false (Utilities|Array|MakeArray _asbp_character) "ForDuration" true "(R=1.000000,G=0.000000,B=0.000000,A=1.000000)" "(R=0.000000,G=1.000000,B=0.000000,A=1.000000)" 1e+01))
  (if (.bblockinghit _outhit)
    (Niagara|SpawnSystematLocation "/Game/Multiplayer_FPS/FX/NS_Burst.NS_Burst" (.location _outhit))
    (if (Utilities|DoesObjectImplementInterface (.hitactor _outhit) "/Game/Multiplayer_FPS/Blueprints/BI_Damage.BI_Damage_C")
      (Class|BIDamage|TakeDamage(Message) (.hitactor _outhit)))))

(event EventBeginPlay)

(event Collision|EventActorBeginOverlap
  (params (OtherActor :type Actor%20Object%20Reference)))

(event EventTick
  (params (DeltaSeconds :type Float%20%28single-precision%29)))

(fn ConstructionScript)